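; Blueprint for the MourningAix enemy character, which sets up its enemy UI when play begins.
; BeginPlay creates the widget class from GetEnemyUIForHUD, pins it to the top center of the player screen and initializes it with this enemy.
; It then casts the ParryWidget component's widget to WWUserWidget and binds it to the same enemy.
; The Blueprint's graphs hold no other active logic.
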(event `self.ReceiveBeginPlay`
  (bind _returnvalue_x (`KismetMathLibrary.BreakVector2D` (`WidgetLayoutLibrary.GetViewportSize`)))
  (bind _returnvalue (`self.GetEnemyUIForHUD`))
  (bind _returnvalue_2 (`|CreateWidget` _returnvalue))
  (`UserWidget.AddToPlayerScreen` _returnvalue_2 0)
  (`UserWidget.SetPositionInViewport` _returnvalue_2 (`KismetMathLibrary.MakeVector2D` (/ _returnvalue_x 2.0)) true)
  (`UserWidget.SetAlignmentInViewport` _returnvalue_2 (0.5 0.0))
  (`WWUserWidget.InitEnemyCreateWidget` _returnvalue_2 self)
  (bind _aswwuser_widget (cast `WWUserWidget` (`WidgetComponent.GetWidget` (`self.ParryWidget`))))
  (`WWUserWidget.InitEnemyCreateWidget` _aswwuser_widget self))

(fn `UserConstructionScript`)