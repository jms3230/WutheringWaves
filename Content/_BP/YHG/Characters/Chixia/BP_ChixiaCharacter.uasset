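; Playable character Blueprint for Chixia, a dual-pistol character.
; BeginPlay hides the left and right pistol components.
; CheckFirstPossessAndInitialize sets a one-time ChixiaInitialize flag once the controller casts to BP_WWPlayerController and has a valid PlayerState.
; Its InitializeAttributeSet call with base combat stats is disconnected, so the function only sets the flag.
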(event `self.ReceiveBeginPlay`
  (`SceneComponent.SetVisibility` (`self.LeftPistol`) false false)
  (`SceneComponent.SetVisibility` (`self.RightPistol`) false false))

(fn `CheckFirstPossessAndInitialize`
  (if (`self.ChixiaInitialize`)
    (return)
    (else
      (bind _asbp_wwplayer_controller (cast `/Game/_BP/YHG/PlayerControllers/BP_WWPlayerController` (`self.GetController`)))
      (`/Engine/EditorBlueprintResources/StandardMacros.IsValid` (`Controller.PlayerState` _asbp_wwplayer_controller)
        (:`Is Valid`
          (set `self.ChixiaInitialize` true)
          (return))))))

(fn `UserConstructionScript`)