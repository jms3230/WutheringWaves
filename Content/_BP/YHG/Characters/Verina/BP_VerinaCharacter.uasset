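; Character Blueprint for Verina, a playable character with an air combo counter.
; BeginPlay hides the Rectifier component, and Tick calls the parent, then resets the air combo count whenever she is grounded.
; A first-possession check sets a one-time initialization flag once the BP_WWPlayerController has a valid PlayerState.
; Its attribute-set initialization with Verina's base stats, cooldowns and energy values is disconnected, so it never runs.
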(event `self.ReceiveBeginPlay`
  (`SceneComponent.SetVisibility` (`self.Rectifier`) false false))

(event `self.ReceiveTick`
  (params (DeltaSeconds :type "Float (single-precision)"))
  (`parent.ReceiveTick` DeltaSeconds)
  (if (`self.bIsGrounded`)
    (set `self.VerinaAirComboCount` 0)))

(fn `CheckFirstPossessAndInitialize`
  (if (`self.VerinaInitialize`)
    (return)
    (else
      (bind _asbp_wwplayer_controller (cast `/Game/_BP/YHG/PlayerControllers/BP_WWPlayerController` (`self.GetController`)))
      (`/Engine/EditorBlueprintResources/StandardMacros.IsValid` (`Controller.PlayerState` _asbp_wwplayer_controller)
        (:`Is Valid`
          (set `self.VerinaInitialize` true)
          (return))))))

(fn `UserConstructionScript`)