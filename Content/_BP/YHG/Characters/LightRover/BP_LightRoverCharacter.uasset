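; Playable Light Rover character Blueprint that sets up the character's starting state and its link to the player HUD.
; BeginPlay hides the sword and scabbard, seeds the attribute set with hardcoded combat, cooldown and energy stats, then links to the WW player controller's HUD widget as Rover.
; CheckFirstPossessAndInitialize repeats the HUD link until it succeeds once, guarded by a flag.
; An alternate attribute setup in that function, starting at half health, is disconnected.
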(event `self.ReceiveBeginPlay`
  (`SceneComponent.SetVisibility` (`self.Scabbard`) false false)
  (`SceneComponent.SetVisibility` (`self.Sword`) false false)
  (`self.InitializeAttributeSet` 912.0 912.0 30.0 30.0 112.0 112.0 100.0 100.0 5.0 5.0 150.0 150.0 6.0 6.0 20.0 20.0 125.0 125.0 100.0 100.0 100.0 100.0)
  (bind _asbp_wwplayer_controller (cast `/Game/_BP/YHG/PlayerControllers/BP_WWPlayerController` (`self.GetController`)))
  (bind _widget_playerhud (`/Game/_BP/YHG/PlayerControllers/BP_WWPlayerController.Widget_PlayerHUD` _asbp_wwplayer_controller))
  (`/Engine/EditorBlueprintResources/StandardMacros.IsValid` _widget_playerhud
    (:`Is Valid`
      (`/Game/_BP/KMJ/Widget/HUD/WBP_PlayerHUD.LinkPawnToUI` _widget_playerhud "Rover"))))

(fn `CheckFirstPossessAndInitialize`
  (if (`self.LightRoverInitialize`)
    (return)
    (else
      (bind _asbp_wwplayer_controller (cast `/Game/_BP/YHG/PlayerControllers/BP_WWPlayerController` (`self.GetController`)))
      (bind _widget_playerhud (`/Game/_BP/YHG/PlayerControllers/BP_WWPlayerController.Widget_PlayerHUD` _asbp_wwplayer_controller))
      (`/Engine/EditorBlueprintResources/StandardMacros.IsValid` _widget_playerhud
        (:`Is Valid`
          (`/Game/_BP/KMJ/Widget/HUD/WBP_PlayerHUD.LinkPawnToUI` _widget_playerhud "Rover")
          (set `self.LightRoverInitialize` true)
          (return))))))

(fn `UserConstructionScript`)